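; Mod Blueprint that revives dead players by turning spectators back into playable characters.
; Mod buttons toggle auto-revive, revive player 0, or revive all players in indices 0 to 15.
; Revival finds characterless players with a BP_Spectator pawn, destroys that pawn and calls RestartPlayer on the game mode.
; Auto-revive runs from Tick through a custom loop macro whose short start Delay throttles the scan.
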(event EventTick
  (params (DeltaSeconds :type Float%20%28single-precision%29))
  (if (Variables|IsCustomMod|GetIsAutoRevive)
    (Utilities|AutoRevivalUpdate)))

(fn ConstructionScript
  (|CallParentFunction))

(fn ModButtonWasPressed
  (params (FunctionIndex :type Integer))
  (switch int FunctionIndex
    (:0
      (bind _output_get (Variables|IsCustomMod|SetIsAutoRevive (not (Variables|IsCustomMod|GetIsAutoRevive))))
      (CallFunction|ModPrint (Utilities|String|Append "Auto Revive: " (Utilities|String|ToString(Boolean) _output_get)) false false false))
    (:1
      (Utilities|ReviveSelf))
    (:2
      (Utilities|ReviveAll))))